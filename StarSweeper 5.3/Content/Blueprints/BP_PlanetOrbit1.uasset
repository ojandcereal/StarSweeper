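; Configurable orbiting-planet Blueprint that sets up a planet mesh circling the actor through rotating movement.
; On BeginPlay it offsets the Planet component by the OrbitRadius vector, assigns its mesh and applies a uniform world scale.
; It then passes RotationRate to the RotatingMovement component, so rotation carries the offset planet around without Tick logic.
; The construction script is empty, so these settings take effect only at runtime.
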(event `self.ReceiveBeginPlay`
  (bind _scaleofplanet (`self.ScaleOfPlanet`))
  (`SceneComponent.K2_SetRelativeLocation` (`self.Planet`) (`self.OrbitRadius`) false false)
  (`StaticMeshComponent.SetStaticMesh` (`self.Planet`) (`self.PlanetMesh`))
  (`SceneComponent.SetWorldScale3D` (`self.Planet`) (`KismetMathLibrary.MakeVector` _scaleofplanet _scaleofplanet _scaleofplanet))
  (set `RotatingMovementComponent.RotationRate` (`self.Rotation Rate`) (`self.RotatingMovement`)))

(fn `UserConstructionScript`)