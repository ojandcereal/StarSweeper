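; BP_Planet is a planet actor that pulls the third-person character toward its surface component while inside its outer collision field.
; Outer collision overlaps toggle a single InGravField flag shared by all overlapping actors.
; While it is set, a Delay-driven loop, rather than Tick, repeatedly passes the normalized direction toward PlanetSurface to the character's AddGrav.
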(event `self.PlanetColOuter.OnComponentEndOverlap`
  (params (OverlappedComponent :type "PrimitiveComponent Object Reference") (OtherActor :type "Actor Object Reference") (OtherComp :type "PrimitiveComponent Object Reference") (OtherBodyIndex :type Integer))
  (set `self.InGravField?` false))

(event `self.PlanetColOuter.OnComponentBeginOverlap`
  (params (OverlappedComponent :type "PrimitiveComponent Object Reference") (OtherActor :type "Actor Object Reference") (OtherComp :type "PrimitiveComponent Object Reference") (OtherBodyIndex :type Integer) (bFromSweep :type Boolean) (SweepResult :type "HitResult Structure (by ref)"))
  (set `self.InGravField?` true)
  (if (`self.InGravField?`) :!label _label
    (bind _output_get (set `self.UnitGrav` (`KismetMathLibrary.Normal` (- (`SceneComponent.K2_GetComponentLocation` (`self.PlanetSurface`)) (`SceneComponent.K2_GetComponentLocation` (`Actor.RootComponent` OtherActor))))))
    (bind _asbp_third_person_character (cast `/Game/ThirdPerson/Blueprints/BP_ThirdPersonCharacter` OtherActor))
    (`/Game/ThirdPerson/Blueprints/BP_ThirdPersonCharacter.AddGrav` _asbp_third_person_character _output_get)
    (`KismetSystemLibrary.Delay` 0.001)
    (goto _label)))

(fn `UserConstructionScript`)