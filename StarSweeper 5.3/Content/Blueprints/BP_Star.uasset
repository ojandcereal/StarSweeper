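; BP_Star is a star pickup actor that the player collects by left-clicking while standing in its collision volume.
; Overlap events on Col enable or disable input on the actor and track whether the player character is inside.
; On click, if the BP_ThirdPersonCharacter has no star, it calls EquipStar on that character with the star mesh, then destroys itself.
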(event `self.Col.OnComponentBeginOverlap`
  (params (OverlappedComponent :type "PrimitiveComponent Object Reference") (OtherActor :type "Actor Object Reference") (OtherComp :type "PrimitiveComponent Object Reference") (OtherBodyIndex :type Integer) (bFromSweep :type Boolean) (SweepResult :type "HitResult Structure (by ref)"))
  (if (== OtherActor (`GameplayStatics.GetPlayerCharacter` 0))
    (`self.EnableInput` (`GameplayStatics.GetPlayerController` 0))
    (set `self.InCol` true)))

(event `self.Col.OnComponentEndOverlap`
  (params (OverlappedComponent :type "PrimitiveComponent Object Reference") (OtherActor :type "Actor Object Reference") (OtherComp :type "PrimitiveComponent Object Reference") (OtherBodyIndex :type Integer))
  (if (== OtherActor (`GameplayStatics.GetPlayerCharacter` 0))
    (`self.DisableInput` (`GameplayStatics.GetPlayerController` 0))
    (set `self.InCol` false)))

(event `Key|LeftMouseButton`
  (params (Key :type "Key Structure"))
  (:`Pressed`
    (if (`self.InCol`)
      (bind _asbp_third_person_character (cast `/Game/ThirdPerson/Blueprints/BP_ThirdPersonCharacter` (stale `self.Col.OnComponentEndOverlap` OtherActor)))
      (if (not (`/Game/ThirdPerson/Blueprints/BP_ThirdPersonCharacter.HasStar?` _asbp_third_person_character))
        (`/Game/ThirdPerson/Blueprints/BP_ThirdPersonCharacter.EquipStar` _asbp_third_person_character "/Game/Content/Misc/Star.Star" "None")
        (`self.K2_DestroyActor`)
        (set `self.InCol` false)))))

(fn `UserConstructionScript`)