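; BP_Rake is an interactable rake actor that the player can equip by left-clicking while near it.
; A sphere overlap with the player character enables input on the actor and sets an InCol flag; leaving reverses both.
; The click casts the begin-overlap's OtherActor to BP_ThirdPersonCharacter and calls its EquipBroom function with a None socket name.
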(event `self.Sphere.OnComponentBeginOverlap`
  (params (OverlappedComponent :type "PrimitiveComponent Object Reference") (OtherActor :type "Actor Object Reference") (OtherComp :type "PrimitiveComponent Object Reference") (OtherBodyIndex :type Integer) (bFromSweep :type Boolean) (SweepResult :type "HitResult Structure (by ref)"))
  (if (== (`GameplayStatics.GetPlayerCharacter` 0) OtherActor)
    (`self.EnableInput` (`GameplayStatics.GetPlayerController` 0))
    (set `self.InCol` true)))

(event `self.Sphere.OnComponentEndOverlap`
  (params (OverlappedComponent :type "PrimitiveComponent Object Reference") (OtherActor :type "Actor Object Reference") (OtherComp :type "PrimitiveComponent Object Reference") (OtherBodyIndex :type Integer))
  (if (== (`GameplayStatics.GetPlayerCharacter` 0) OtherActor)
    (`self.DisableInput` (`GameplayStatics.GetPlayerController` 0))
    (set `self.InCol` false)))

(event `Key|LeftMouseButton`
  (params (Key :type "Key Structure"))
  (:`Pressed`
    (if (`self.InCol`)
      (bind _asbp_third_person_character (cast `/Game/ThirdPerson/Blueprints/BP_ThirdPersonCharacter` (stale `self.Sphere.OnComponentEndOverlap` OtherActor)))
      (`/Game/ThirdPerson/Blueprints/BP_ThirdPersonCharacter.EquipBroom` _asbp_third_person_character null "None"))))

(fn `UserConstructionScript`)